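; Sphere actor that puts the third-person character into a gravity lock when the character overlaps it.
; On overlap it sets the character's InGravLock flag and zeroes its ForceGravity vector.
; It also adds a counter-velocity to the capsule's physics velocity, weighted more heavily on Z, and clears accumulated movement forces before and after.
; Nothing here releases the lock when the overlap ends.
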(event EventBeginPlay)

(event EventTick
  (params (DeltaSeconds :type Float%20%28single-precision%29)))

(event Collision|EventActorBeginOverlap
  (params (OtherActor :type Actor%20Object%20Reference))
  (bind _asbp_third_person_character (Utilities|Casting|CastToBP_ThirdPersonCharacter OtherActor))
  (bind _output_get (Variables|Default|SetCharctr _asbp_third_person_character))
  (Variables|/Game/ThirdPerson/Blueprints/BP_ThirdPersonCharacter.BP_ThirdPersonCharacter_C|SetInGravLock _output_get true)
  (Variables|/Game/ThirdPerson/Blueprints/BP_ThirdPersonCharacter.BP_ThirdPersonCharacter_C|SetForceGravity _output_get "0, 0, 0")
  (Pawn|Components|CharacterMovement|ClearAccumulatedForces (Variables|/Script/Engine.Character|GetCharacterMovement _asbp_third_person_character))
  (bind _returnvalue (Physics|GetPhysicsLinearVelocity (Variables|/Script/Engine.Character|GetCapsuleComponent _output_get) "None"))
  (bind _returnvalue_2 (Physics|GetPhysicsLinearVelocity (Variables|/Script/Engine.Character|GetCapsuleComponent _output_get) "None"))
  (Physics|SetPhysicsLinearVelocity (Variables|/Script/Engine.Character|GetCapsuleComponent _output_get) (- _returnvalue (* _returnvalue_2 "2.000000,2.000000,4.000000")) true "None")
  (Pawn|Components|CharacterMovement|ClearAccumulatedForces (Variables|/Script/Engine.Character|GetCharacterMovement _asbp_third_person_character)))

(fn ConstructionScript)